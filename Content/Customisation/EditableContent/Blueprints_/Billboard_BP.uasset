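; Editable billboard actor that downloads its image from the hosting platform, keyed by object name, into a dynamic material.
; An ImageEdit_UMG widget fades in when the local player overlaps; its buttons send a Pixel Streaming edit request or delete the image via the API.
; A looping timer re-downloads the image, dropping to a short delay when an "updated" message for its ID arrives, then returning to slow polling.
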(event `GetSettings`
  (bind _platformdata_eventid (break `PMPlatformData` (`PixelMaxHostingSubsystem.PlatformData` (subsystem `PixelMaxHostingSubsystem`))))
  ;[1 0.5661 0] GetSettings
  (bind _output_get (set `self.ID` (`KismetSystemLibrary.GetObjectName` self)))
  (bind _texture (`AsyncTaskDownloadImage.DownloadImage` (`KismetStringLibrary.Concat_StrStr` (`self.PlatformDomain`) "/worlds/" _platformdata_eventid "/location/" _output_get "/image"))
    (:`OnSuccess`
      (`MaterialInstanceDynamic.SetTextureParameterValue` (`self.Image_Ref`) "DLImage" _texture))))

(event `self.ReceiveBeginPlay`
  ;[0 0.2095 1] BeginPlay & Binding
  (`|ExecutionSequence`
    (:`then_0`
      (set `self.PlatformDomain` (`PixelMaxHostingSubsystem.PlatformDomain` (subsystem `PixelMaxHostingSubsystem`)))
      (`self.GetSettings`)
      (bind _asimage_edit_umg (cast `/Game/Customisation/EditableContent/Widgets/ImageEdit_UMG` (`WidgetComponent.GetUserWidgetObject` (`self.Settings`))))
      (set `self.SettingsRef` _asimage_edit_umg)
      (`self.SetWidgetStyle`))
    (:`then_1`
      (`self.BindWidget`)
      (`self.BindDelete`))
    (:`then_2`
      (add `PixelStreamingInput.OnInputEvent` (`self.GetComponentByClass` (`GameplayStatics.GetPlayerController` 0) "/Script/PixelStreaming.PixelStreamingInput") (delegate `Getdata`))
      (`self.StartTimer`))))

(event `Getdata`
  (params (Descriptor :type String))
  (bind _returnvalue (`self.GetComponentByClass` (`GameplayStatics.GetPlayerController` 0) "/Script/PixelStreaming.PixelStreamingInput"))
  ;[0.1854 1 0] ResetTimer
  (if (`KismetStringLibrary.EqualEqual_StrStr` (`PixelStreamingInput.GetJsonStringValue` _returnvalue Descriptor "id") (`self.ID`))
    (if (`KismetStringLibrary.EqualEqual_StrStr` (`PixelStreamingInput.GetJsonStringValue` _returnvalue Descriptor "type") "updated")
      (`self.ResetTimer`))))

(event `BindWidget`
  ;[1 0 0.5104] BindWidget
  (bind _asimage_edit_umg (cast `/Game/Customisation/EditableContent/Widgets/ImageEdit_UMG` (`WidgetComponent.GetUserWidgetObject` (`self.Settings`))))
  (add `/Game/Customisation/EditableContent/Widgets/ImageEdit_UMG.Interact_` _asimage_edit_umg (delegate `EditImageSend`)))

(event `EditImageSend`
  ;[1 1 1] EditWallSend
  (`PixelStreamingInput.SendPixelStreamingResponse` (`self.GetComponentByClass` (`GameplayStatics.GetPlayerController` 0) "/Script/PixelStreaming.PixelStreamingInput") (`KismetStringLibrary.Concat_StrStr` "{\"type\": \"edit\", \"format\": \"image\", \"id\": \"" (`self.ID`) "\", \"res\": {\"x\": \"" (`KismetStringLibrary.Conv_IntToString` (`self.X Res`)) "\", \"y\": \"" (`KismetStringLibrary.Conv_IntToString` (`self.Y Res`)) "\"}}")))

(event `StartTimer`
  ;[0 0.8372 1] StartTimer
  (bind _returnvalue (`KismetSystemLibrary.K2_SetTimerDelegate` (delegate `ApplySettings`) (`self.UpdateTime`) true 2.0))
  (bind _output_get (set `self.Timer` _returnvalue)))

(event `ResetTimer`
  ;[0 0.8372 1] StartTimer
  (`KismetSystemLibrary.K2_ClearAndInvalidateTimerHandle` (`self.Timer`))
  (set `self.UpdateTime` 1.0)
  (`self.StartTimer`))

(event `ApplySettings`
  ;[0 0.8372 1] StartTimer
  (`self.GetSettings`)
  (`KismetSystemLibrary.K2_ClearAndInvalidateTimerHandle` (stale `StartTimer` _output_get))
  (set `self.UpdateTime` 240.0)
  (`self.StartTimer`))

(event `BindDelete`
  ;[1 1 1] Delete
  (bind _asimage_edit_umg (cast `/Game/Customisation/EditableContent/Widgets/ImageEdit_UMG` (`WidgetComponent.GetUserWidgetObject` (`self.Settings`))))
  (add `/Game/Customisation/EditableContent/Widgets/ImageEdit_UMG.Delete_` _asimage_edit_umg (delegate `Delete`)))

(event `Delete`
  (bind _platformdata_eventid (break `PMPlatformData` (`PixelMaxHostingSubsystem.PlatformData` (subsystem `PixelMaxHostingSubsystem`))))
  ;[1 1 1] Delete
  (`MaterialInstanceDynamic.SetTextureParameterValue` (`self.Image_Ref`) "DLImage" "/Game/Customisation/EditableContent/Materials/SourceTextures/Def_Billboard.Def_Billboard")
  (`PixelMaxAPIRequest.AsyncAPIRequest` (`KismetStringLibrary.Concat_StrStr` (`self.PlatformDomain`) "/worlds/" _platformdata_eventid "/location/" (`KismetSystemLibrary.GetObjectName` self) "/image") "DELETE"))

(event `self.PlayerCheck.OnComponentBeginOverlap`
  (params (OverlappedComponent :type "PrimitiveComponent Object Reference") (OtherActor :type "Actor Object Reference") (OtherComp :type "PrimitiveComponent Object Reference") (OtherBodyIndex :type Integer) (bFromSweep :type Boolean) (SweepResult :type "HitResult Structure (by ref)"))
  (bind _settings (`self.Settings`))
  (bind _instigator (`Actor.Instigator` OtherActor))
  ;[1 0 0.01386] FadeWidget
  (`/Engine/EditorBlueprintResources/StandardMacros.IsValid` _instigator
    (:`Is Valid`
      (if (`Pawn.IsLocallyControlled` _instigator)
        (`SceneComponent.SetHiddenInGame` _settings false false)
        (bind _asimage_edit_umg (cast `/Game/Customisation/EditableContent/Widgets/ImageEdit_UMG` (`WidgetComponent.GetUserWidgetObject` _settings)))
        (bind (_direction _newtrack_0) (`Timeline|Timeline_0` :!via `PlayFromStart`)
          (:`Update`
            (`Widget.SetRenderOpacity` _asimage_edit_umg _newtrack_0)))))))

(event `self.PlayerCheck.OnComponentEndOverlap`
  (params (OverlappedComponent :type "PrimitiveComponent Object Reference") (OtherActor :type "Actor Object Reference") (OtherComp :type "PrimitiveComponent Object Reference") (OtherBodyIndex :type Integer))
  (bind _settings (`self.Settings`))
  (bind _instigator (`Actor.Instigator` OtherActor))
  ;[1 0 0.01386] FadeWidget
  (`/Engine/EditorBlueprintResources/StandardMacros.IsValid` _instigator
    (:`Is Valid`
      (if (`Pawn.IsLocallyControlled` _instigator)
        (bind _asimage_edit_umg (cast `/Game/Customisation/EditableContent/Widgets/ImageEdit_UMG` (`WidgetComponent.GetUserWidgetObject` _settings)))
        (bind (_direction _newtrack_0) (`Timeline|Timeline_1` :!via `ReverseFromEnd`)
          (:`Update`
            (`Widget.SetRenderOpacity` _asimage_edit_umg _newtrack_0))
          (:`Finished`
            (`SceneComponent.SetHiddenInGame` _settings true false)))))))

(fn `SetWidgetStyle`
  (bind _asimage_edit_umg (cast `/Game/Customisation/EditableContent/Widgets/ImageEdit_UMG` (`WidgetComponent.GetUserWidgetObject` (`self.Settings`))))
  (`Button.SetStyle` (`/Game/Customisation/EditableContent/Widgets/ImageEdit_UMG.Interact` _asimage_edit_umg) (`self.Interact Style`))
  (`Button.SetStyle` (`/Game/Customisation/EditableContent/Widgets/ImageEdit_UMG.Delete` _asimage_edit_umg) (`self.Delete Style`)))

(fn `UserConstructionScript`
  (bind _settings (`self.Settings`))
  (bind _returnvalue (`PrimitiveComponent.CreateDynamicMaterialInstance` (`self.Image`) 0 "/Game/Customisation/EditableContent/Materials/DynamicMasterBillboard.DynamicMasterBillboard" "DMB"))
  (set `self.Image_Ref` _returnvalue)
  (if (`self.Widget?`)
    (`SceneComponent.SetVisibility` _settings true false)
    (else
      (`SceneComponent.SetVisibility` _settings false false))))