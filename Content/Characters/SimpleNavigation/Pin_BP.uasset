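; Navigation pin actor with a world-space UI_Pin widget that plays its SetPin animation on spawn and turns toward the player camera every tick.
; When the locally controlled pawn overlaps the Sphere, the animation plays in reverse, and overlapping the Box destroys the pin.
; Interacting with the pin stops the player controller's movement and destroys it.
; A timer also removes the pin after a fixed lifespan.
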(event `self.Box.OnComponentBeginOverlap`
  (params (OverlappedComponent :type "PrimitiveComponent Object Reference") (OtherActor :type "Actor Object Reference") (OtherComp :type "PrimitiveComponent Object Reference") (OtherBodyIndex :type Integer) (bFromSweep :type Boolean) (SweepResult :type "HitResult Structure (by ref)"))
  ;[0.905 1 0] Player Collision
  (bind _aspawn (cast `Pawn` OtherActor))
  (if (`Pawn.IsLocallyControlled` _aspawn)
    (`self.K2_DestroyActor`)))

(event `self.Sphere.OnComponentBeginOverlap`
  (params (OverlappedComponent :type "PrimitiveComponent Object Reference") (OtherActor :type "Actor Object Reference") (OtherComp :type "PrimitiveComponent Object Reference") (OtherBodyIndex :type Integer) (bFromSweep :type Boolean) (SweepResult :type "HitResult Structure (by ref)"))
  ;[0.905 1 0] Player Collision
  (bind _aspawn (cast `Pawn` OtherActor))
  (if (`Pawn.IsLocallyControlled` _aspawn)
    (set `self.Play Mode` "Reverse")
    (`self.Animation`)))

(event `Animation`
  ;[0 0.1436 1] Animation/Playertracking
  (bind _asui_pin (cast `/Game/Characters/SimpleNavigation/UI_Nav/UI_Pin` (`WidgetComponent.GetUserWidgetObject` (`self.Widget`))))
  (`UserWidget.PlayAnimation` _asui_pin (`/Game/Characters/SimpleNavigation/UI_Nav/UI_Pin.SetPin` _asui_pin) 0.0 1 (`self.Play Mode`) 1.0 false))

(event `self.ReceiveTick`
  (params (DeltaSeconds :type "Float (single-precision)"))
  (bind _widget (`self.Widget`))
  ;[0 0.1436 1] Animation/Playertracking
  (`SceneComponent.K2_SetWorldRotation` _widget (`KismetMathLibrary.FindLookAtRotation` (`SceneComponent.K2_GetComponentLocation` _widget) (`PlayerCameraManager.GetCameraLocation` (`GameplayStatics.GetPlayerCameraManager` 0))) false false))

(event `/Game/Hosting/PlatformContent/InteractInterface.Interact`
  (params (`Actor to Interact` :type "Actor Object Reference"))
  ;[1 0 0.04706] Stop Movement
  (`Controller.StopMovement` (`GameplayStatics.GetPlayerController` 0))
  (`self.K2_DestroyActor`))

(event `self.ReceiveBeginPlay`
  ;[0.1644 1 0] BeginPlay/Lifespan
  (`KismetSystemLibrary.K2_SetTimerDelegate` (delegate `Lifespan`) 20.0)
  (`self.Animation`))

(event `Lifespan`
  ;[0.1644 1 0] BeginPlay/Lifespan
  (`self.K2_DestroyActor`))

(fn `UserConstructionScript`)