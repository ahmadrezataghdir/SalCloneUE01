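; Player controller for Clementine that routes input to player 0's character for moving, looking, jumping, crouching and running.
; Movement follows control yaw, and gamepad look scales with base rates and delta time, while mouse look is unscaled.
; ForwardMotion feeds both forward and right movement and LookupRate both pitch and yaw; RightMotion and TurnRate are empty.
; Run swaps MaxWalkSpeed between run and walk speeds, printing debug speed readouts.
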(event `InputAction|Jump`
  (params (Key :type "Key Structure"))
  (bind _returnvalue (`GameplayStatics.GetPlayerCharacter` 0))
  ;[1 0.3146 0.5914] Jumping
  (:`Pressed`
    (`Character.Jump` _returnvalue))
  (:`Released`
    (`Character.StopJumping` _returnvalue)))

(event `InputAxis|LookUp(Mouse)Pitch`
  (params (AxisValue :type "Float (single-precision)"))
  ;[1 1 1] Mouse Controls
  (`Pawn.AddControllerPitchInput` (`GameplayStatics.GetPlayerPawn` 0) AxisValue))

(event `InputAxis|Turn(Mouse)YAW`
  (params (AxisValue :type "Float (single-precision)"))
  ;[1 1 1] Mouse Controls
  (`Pawn.AddControllerYawInput` (`GameplayStatics.GetPlayerPawn` 0) AxisValue))

(event `InputAction|Crouch`
  (params (Key :type "Key Structure"))
  (bind _returnvalue (`GameplayStatics.GetPlayerCharacter` 0))
  ;[1 1 1] Crouching Control
  (:`Pressed`
    (`Character.Crouch` _returnvalue))
  (:`Released`
    (`Character.UnCrouch` _returnvalue)))

(event `InputAxis|ForwardMotion`
  (params (AxisValue :type "Float (single-precision)"))
  (bind _returnvalue (`GameplayStatics.GetPlayerPawn` 0))
  (bind _returnvalue_2 (`self.GetControlRotation`))
  ;[1 1 1] Movement
  (`Pawn.AddMovementInput` _returnvalue (`KismetMathLibrary.GetForwardVector` (`KismetMathLibrary.MakeRotator` 0.0 0.0 (.yaw _returnvalue_2))) AxisValue false)
  (`Pawn.AddMovementInput` _returnvalue (`KismetMathLibrary.GetRightVector` (`KismetMathLibrary.MakeRotator` 0.0 0.0 (.yaw _returnvalue_2))) (stale `InputAxis|RightMotion` AxisValue) false))

(event `InputAxis|RightMotion`
  (params (AxisValue :type "Float (single-precision)"))
  ;[1 1 1] Movement
)

(event `InputAxis|LookupRate(GamePad)Pitch`
  (params (AxisValue :type "Float (single-precision)"))
  (bind _returnvalue (`GameplayStatics.GetPlayerPawn` 0))
  (`Pawn.AddControllerPitchInput` _returnvalue (* AxisValue (`GameplayStatics.GetWorldDeltaSeconds`) (`self.BaseLookupRate`)))
  (`Pawn.AddControllerYawInput` _returnvalue (* (stale `InputAxis|TurnRate(Gamepad)YAW` AxisValue) (`GameplayStatics.GetWorldDeltaSeconds`) (`self.BaseTurnRate`))))

(event `InputAxis|TurnRate(Gamepad)YAW`
  (params (AxisValue :type "Float (single-precision)")))

(event `InputAction|Run`
  (params (Key :type "Key Structure"))
  (bind _returnvalue (`GameplayStatics.GetPlayerPawn` 0))
  (bind _charactermovement (`Character.CharacterMovement` (`GameplayStatics.GetPlayerCharacter` 0)))
  (:`Pressed`
    (bind _output_get (set `CharacterMovementComponent.MaxWalkSpeed` (`self.RunSpeed`) _charactermovement))
    (`KismetSystemLibrary.PrintString` (`KismetStringLibrary.Conv_DoubleToString` _output_get) true true (struct :`R` 1.0 :`G` 0.829836 :`A` 1.0))
    (`KismetSystemLibrary.PrintString` (`KismetStringLibrary.Concat_StrStr` "Speed:" (`KismetStringLibrary.Conv_DoubleToString` (`KismetMathLibrary.VSize` (`self.GetVelocity` _returnvalue))))))
  (:`Released`
    (bind _output_get_2 (set `CharacterMovementComponent.MaxWalkSpeed` (`self.WalkSpeed`) _charactermovement))
    (`KismetSystemLibrary.PrintString` (`KismetStringLibrary.Conv_DoubleToString` _output_get_2) true true (struct :`R` 1.0 :`B` 0.386642 :`A` 1.0))
    (`KismetSystemLibrary.PrintString` (`KismetStringLibrary.Concat_StrStr` "Speed:" (`KismetStringLibrary.Conv_DoubleToString` (`KismetMathLibrary.VSize` (`self.GetVelocity` _returnvalue)))))))

(fn `UserConstructionScript`)