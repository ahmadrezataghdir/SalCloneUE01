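; NPC spawner actor that fills the area around itself with BP_NPC_M characters once the player controller comes within SpawnerRange.
; BeginPlay enables Tick after a random delay, and Tick checks the distance, printing it when in range.
; A DoOnce-guarded delayed loop spawns at random reachable navmesh points nearby until SpawnedNpcCount reaches RequiredNpcCount, then resets.
; The count is never decremented here.
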(event `self.ReceiveBeginPlay`
  (`KismetSystemLibrary.Delay` (`KismetMathLibrary.RandomFloatInRange` 0.5 2.0))
  (`self.SetActorTickEnabled` true))

(event `self.ReceiveTick`
  (params (DeltaSeconds :type "Float (single-precision)"))
  (bind _returnvalue (`KismetMathLibrary.Vector_Distance` (`self.K2_GetActorLocation` (`GameplayStatics.GetPlayerController` 0)) (`self.K2_GetActorLocation`)))
  (if (< _returnvalue (`self.spawner_range`))
    (`KismetSystemLibrary.PrintString` (`KismetStringLibrary.Conv_DoubleToString` _returnvalue))
    (`self.Spawned NPCs`)))

(event `Spawned NPCs`
  (`/Engine/EditorBlueprintResources/StandardMacros.DoOnce` false :!label _label
    (:`Completed`
      (if (> (`self.required_npc_count`) (`self.spawned_npc_count`)) :!label _label_2
        (bind _returnvalue (`|SpawnActorFromClass` "/Game/Characters/NPC/AI2/Blueprints/BP_NPC_M.BP_NPC_M_C" (`KismetMathLibrary.MakeTransform` (`NavigationSystemV1.K2_GetRandomReachablePointInRadius` (`self.K2_GetActorLocation`) 500.0 null null)) "AdjustIfPossibleButAlwaysSpawn" "MultiplyWithRoot" null null))
        (`/Engine/EditorBlueprintResources/StandardMacros.IsValid` _returnvalue
          (:`Is Valid`
            (`/Engine/EditorBlueprintResources/StandardMacros.IncrementInt` (`self.spawned_npc_count`)
              (:`  `
                (`KismetSystemLibrary.Delay` 0.2)
                (goto _label_2)))))
        (else
          (goto _label :!via `Reset`))))))

(fn `UserConstructionScript`)