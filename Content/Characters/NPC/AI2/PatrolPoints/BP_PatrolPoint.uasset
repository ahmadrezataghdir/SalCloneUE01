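; BP_PatrolPoint is a patrol node, filed under NPC AI, that links to other points through next and previous lists.
; Its construction script clears the Cube's child components, then draws a spline to each linked point as a visual aid.
; Next links are green and previous links red, offset to opposite sides so they stay distinguishable.
; GetNextPatrolPoint returns a random point from either list according to travel direction.
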(fn `DrawSplines`
  (params (Points :type "Array of /Game/Characters/NPC/AI2/PatrolPoints/BP_PatrolPoint Object Reference") (BetweenDistance :type "Float (double-precision)") (`Line Color` :type "LinearColor Structure"))
  (locals (CurrentPoint :type "/Game/Characters/NPC/AI2/PatrolPoints/BP_PatrolPoint Object Reference") (CurrentSpline :type "SplineComponent Object Reference"))
  (bind _cube (`self.Cube`))
  (bind _betweendistance (`local.BetweenDistance`))
  (bind _cube_2 (`self.Cube`))
  (bind _betweendistance_2 (`local.BetweenDistance`))
  (for _array_element Points
    (set `local.CurrentPoint` _array_element)
    ;[1 1 1] Create Spline
    (bind _returnvalue (`AddComponent|NODE_AddSplineComponent-0`))
    (bind _output_get (set `local.CurrentSpline` _returnvalue))
    (`SceneComponent.K2_AttachToComponent` _output_get (`self.Cube`) "None" "SnapToTarget" "KeepRelative" "KeepRelative" true)
    (`SplineComponent.SetUnselectedSplineSegmentColor` (`local.CurrentSpline`) (`local.Line Color`))
    (`SplineComponent.SetLocationAtSplinePoint` (`local.CurrentSpline`) 0 (+ (`SceneComponent.K2_GetComponentLocation` _cube) (* (`SceneComponent.GetRightVector` _cube) _betweendistance) (* (`SceneComponent.GetForwardVector` _cube) _betweendistance)) "World" false)
    (`SplineComponent.SetLocationAtSplinePoint` (`local.CurrentSpline`) 1 (+ (`SceneComponent.K2_GetComponentLocation` (`/Game/Characters/NPC/AI2/PatrolPoints/BP_PatrolPoint.Cube` (`local.CurrentPoint`))) (* (`SceneComponent.GetRightVector` _cube_2) _betweendistance_2) (* (`SceneComponent.GetForwardVector` _cube_2) _betweendistance_2)) "World" true)))

(fn `GetNextPatrolPoint`
  (params (IsForwards :type Boolean))
  (returns (PatrolPoint :type "/Game/Characters/NPC/AI2/PatrolPoints/BP_PatrolPoint Object Reference"))
  (return (`KismetArrayLibrary.Array_Random` (select `bool` IsForwards :`false` (`self.PreviousPoints`) :`true` (`self.NextPoints`)))))

(fn `UserConstructionScript`
  (locals (TotalPoints :type Integer))
  (set `local.TotalPoints` (+ (`KismetArrayLibrary.Array_Length` (`self.NextPoints`)) (`KismetArrayLibrary.Array_Length` (`self.PreviousPoints`))))
  (for _array_element (`SceneComponent.GetChildrenComponents` (`self.Cube`) false)
    (`ActorComponent.K2_DestroyComponent` _array_element))
  (`self.DrawSplines` (`self.NextPoints`) -50.0 (struct :`R` 0.20501 :`G` 1.0 :`B` 0.128417 :`A` 1.0))
  (`self.DrawSplines` (`self.PreviousPoints`) 50.0 (struct :`R` 1.0 :`G` 0.020833 :`B` 0.14615 :`A` 1.0)))