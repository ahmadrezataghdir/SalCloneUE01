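; Game state Blueprint, judging by its name, that keeps a shared pool of available NPCs for other code to draw from.
; The AddAvailableNPC event registers an NPC in the AvailableNPCs array without duplicates.
; GetAvailableNPC removes the first entry, then reads index 0 for its return, so it yields the following NPC rather than the removed one.
; An empty pool returns nothing, and BeginPlay, Tick and the construction script are unused.
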(event `/Game/Characters/NPC/AI2/Blueprints/BPI_NPCManage.AddAvailableNPC`
  (params (NPC :type "Actor Object Reference"))
  (`KismetArrayLibrary.Array_AddUnique` (`self.AvailableNPCs`) NPC))

(fn `GetAvailableNPC`
  (returns (NPC :type "Actor Object Reference"))
  (bind _availablenpcs (`self.AvailableNPCs`))
  (if (> (`KismetArrayLibrary.Array_Length` _availablenpcs) 0)
    (`KismetArrayLibrary.Array_Remove` _availablenpcs)
    (return (`|GetArrayItem` _availablenpcs))
    (else
      (return null))))

(fn `UserConstructionScript`)