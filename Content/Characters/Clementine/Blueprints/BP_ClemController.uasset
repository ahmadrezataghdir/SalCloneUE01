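; Player controller for the Clementine character that handles third-person movement and camera input through Enhanced Input.
; BeginPlay adds the IMC_ThirdPerson mapping context, and input actions drive jump, crouch, camera-relative movement and look on the player pawn.
; Sprint switches MaxWalkSpeed between run and walk speeds, and look applies optional per-axis camera inversion.
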(event `self.ReceiveBeginPlay`
  (bind _returnvalue (subsystem `EnhancedInputLocalPlayerSubsystem`))
  (`/Engine/EditorBlueprintResources/StandardMacros.IsValid` _returnvalue
    (:`Is Valid`
      (`EnhancedInputSubsystemInterface.AddMappingContext` _returnvalue "/Game/Characters/Clementine/InputMapping/IMC_ThirdPerson.IMC_ThirdPerson" 0 (struct)))))

(event `EnhancedInput|/Game/Characters/Clementine/Inputs/INP_Jump`
  (params (ActionValue :type Boolean) (ElapsedSeconds :type "Float (double-precision)") (TriggeredSeconds :type "Float (double-precision)") (InputAction :type "InputAction Object Reference" :default "/Game/Characters/Clementine/Inputs/INP_Jump.INP_Jump"))
  (bind _returnvalue (`GameplayStatics.GetPlayerCharacter` 0))
  (:`Started`
    (`Character.Jump` _returnvalue))
  (:`Completed`
    ;[1 0.3146 0.5914] Jumping
    (`Character.StopJumping` _returnvalue)))

(event `EnhancedInput|/Game/Characters/Clementine/Inputs/INP_Crouch`
  (params (ActionValue :type Boolean) (ElapsedSeconds :type "Float (double-precision)") (TriggeredSeconds :type "Float (double-precision)") (InputAction :type "InputAction Object Reference" :default "/Game/Characters/Clementine/Inputs/INP_Crouch.INP_Crouch"))
  (bind _returnvalue (`GameplayStatics.GetPlayerCharacter` 0))
  ;[1 1 1] Crouching Control
  (:`Triggered`
    (`Character.Crouch` _returnvalue))
  (:`Completed`
    (`Character.UnCrouch` _returnvalue)))

(event `EnhancedInput|/Game/Characters/Clementine/Inputs/INP_MoveAround`
  (params (ActionValue :type "Vector2D Structure") (ElapsedSeconds :type "Float (double-precision)") (TriggeredSeconds :type "Float (double-precision)") (InputAction :type "InputAction Object Reference" :default "/Game/Characters/Clementine/Inputs/INP_MoveAround.INP_MoveAround"))
  (bind _returnvalue (`GameplayStatics.GetPlayerPawn` 0))
  (bind (_returnvalue_roll _returnvalue_pitch _returnvalue_yaw) (`KismetMathLibrary.BreakRotator` (`self.GetControlRotation`)))
  (:`Triggered`
    (`Pawn.AddMovementInput` _returnvalue (`KismetMathLibrary.GetRightVector` (`self.GetControlRotation`)) ActionValue_X false)
    (`Pawn.AddMovementInput` _returnvalue (`KismetMathLibrary.GetForwardVector` (`KismetMathLibrary.MakeRotator` _returnvalue_roll 0.0 _returnvalue_yaw)) ActionValue_Y false)))

(event `EnhancedInput|/Game/Characters/Clementine/Inputs/INP_Sprint`
  (params (ActionValue :type Boolean) (ElapsedSeconds :type "Float (double-precision)") (TriggeredSeconds :type "Float (double-precision)") (InputAction :type "InputAction Object Reference" :default "/Game/Characters/Clementine/Inputs/INP_Sprint.INP_Sprint"))
  (bind _charactermovement (`Character.CharacterMovement` (`GameplayStatics.GetPlayerCharacter` 0)))
  ;[1 1 1] Sprint
  (:`Triggered`
    (set `CharacterMovementComponent.MaxWalkSpeed` (`self.RunSpeed`) _charactermovement))
  (:`Completed`
    (set `CharacterMovementComponent.MaxWalkSpeed` (`self.WalkSpeed`) _charactermovement)))

(event `EnhancedInput|/Game/Characters/Clementine/Inputs/INP_LookAround`
  (params (ActionValue :type "Vector2D Structure") (ElapsedSeconds :type "Float (double-precision)") (TriggeredSeconds :type "Float (double-precision)") (InputAction :type "InputAction Object Reference" :default "/Game/Characters/Clementine/Inputs/INP_LookAround.INP_LookAround"))
  (bind _returnvalue (`GameplayStatics.GetPlayerPawn` 0))
  (:`Triggered`
    (`Pawn.AddControllerYawInput` _returnvalue (* ActionValue_X (`KismetMathLibrary.SelectFloat` -1.0 1.0 (`self.InvertCameraX`))))
    (`Pawn.AddControllerPitchInput` _returnvalue (* ActionValue_Y (`KismetMathLibrary.SelectFloat` -1.0 1.0 (`self.InvertCameraY`))))))

(fn `UserConstructionScript`)