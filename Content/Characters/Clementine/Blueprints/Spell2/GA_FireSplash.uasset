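; Gameplay ability for Clementine's Fire Splash spell, which plays a cast montage and spawns the splash actor at the character's feet.
; Movement is disabled for player 0's character during the montage and set back to walking only when it completes.
; A montage gameplay event triggers the BP_FireSplash spawn midway between the two toe sockets, facing the avatar's rotation.
; The graph never calls EndAbility.
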(event `self.K2_ActivateAbility`
  (`AbilityTask_PlayMontageAndWait.CreatePlayMontageAndWaitProxy` "None" "/Game/Characters/Clementine/Anims/Magic/AN_SpellSplash.AN_SpellSplash"
    (:`then`
      (`CharacterMovementComponent.SetMovementMode` (`Character.CharacterMovement` (`GameplayStatics.GetPlayerCharacter` 0)) "MOVE_None" 0)
      (`AbilityTask_WaitGameplayEvent.WaitGameplayEvent` (struct :`TagName` "Event.Montage.FireSplash") null
        (:`EventReceived`
          (bind _asbp_clem (cast `/Game/Characters/Clementine/Blueprints/BP_Clem` (`self.GetAvatarActorFromActorInfo`)))
          (bind _mesh (`Character.Mesh` _asbp_clem))
          (`|SpawnActorFromClass` "/Game/Characters/Clementine/Blueprints/Spell2/BP_FireSplash.BP_FireSplash_C" (`KismetMathLibrary.MakeTransform` (* (+ (`SceneComponent.GetSocketLocation` _mesh "RightToeBase") (`SceneComponent.GetSocketLocation` _mesh "LeftToeBase")) 0.5) (`Actor.K2_GetActorRotation` _asbp_clem)) "Undefined" "MultiplyWithRoot" null null))))
    (:`OnCompleted`
      (`CharacterMovementComponent.SetMovementMode` (`Character.CharacterMovement` (`GameplayStatics.GetPlayerCharacter` 0)) "MOVE_Walking" 0))))