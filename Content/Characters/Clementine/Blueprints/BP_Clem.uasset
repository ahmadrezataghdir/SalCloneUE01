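; Player character Clementine, who walks on foot and can switch to driving a scooter.
; E, when InsideScooter is set, possesses the scooter pawn and swaps Enhanced Input mapping contexts.
; ActivateRagdoll enables mesh physics, shows a Wasted screen with sound and camera fade, then reloads the Test level after a delay; DeactivateRagdoll restores walking.
; Hotkeys also toggle ragdoll, spawn FireNavMesh and print distance to the NPC spawner.
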(event `self.ReceiveBeginPlay`
  (set `CharacterMovementComponent.MaxWalkSpeed` 180.0 (`self.CharacterMovement`)))

(event `self.OnLanded`
  (params (Hit :type "HitResult Structure (by ref)"))
  (if (`NavMovementComponent.IsFalling` (`self.CharacterMovement`))
    _))

(event `Key|Q`
  (params (Key :type "Key Structure"))
  (:`Pressed`
    (`|SpawnActorFromClass` "/Game/Characters/NPC/AI2/FireNavMesh.FireNavMesh_C" (`SceneComponent.K2_GetComponentToWorld` (`self.Mesh`)) "AlwaysSpawn" "MultiplyWithRoot" null null)))

(event `Key|T`
  (params (Key :type "Key Structure"))
  ;[1 1 1] Not using
)

(event `Key|E`
  (params (Key :type "Key Structure"))
  (bind _returnvalue (`GameplayStatics.GetPlayerController` 0))
  (bind _returnvalue_2 (pcsubsystem `EnhancedInputLocalPlayerSubsystem` _returnvalue))
  ;[1 1 1] Works only when in scooter range, Leaving char control and grabbing scooter control.
  (:`Pressed`
    (if (`self.InsideScooter`)
      (bind _returnvalue_3 (`GameplayStatics.GetActorOfClass` "/Game/Characters/Clementine/Interaction/BP_PawnScooter.BP_PawnScooter_C"))
      (`GameplayStatics.PlaySound2D` "/Engine/VREditor/Sounds/UI/Click_on_Button.Click_on_Button" 1.0 1.0 0.0 null null)
      (`Controller.Possess` _returnvalue _returnvalue_3)
      (`EnhancedInputSubsystemInterface.RemoveMappingContext` _returnvalue_2 "/Game/Characters/Clementine/InputMapping/IMC_ThirdPerson.IMC_ThirdPerson" (struct))
      (`EnhancedInputSubsystemInterface.AddMappingContext` _returnvalue_2 "/Game/Characters/Clementine/InputMapping/IMC_Scooter.IMC_Scooter" 0 (struct))
      (else
        (`KismetSystemLibrary.PrintString` "No Inside Scooter")))))

(event `self.ReceivePossessed`
  (params (NewController :type "Controller Object Reference"))
  ;[1 1 1] Works only when in scooter range, Leaving char control and grabbing scooter control.
  (`EnhancedInputSubsystemInterface.AddMappingContext` (pcsubsystem `EnhancedInputLocalPlayerSubsystem` (`GameplayStatics.GetPlayerController` 0)) "/Game/Characters/Clementine/InputMapping/IMC_ThirdPerson.IMC_ThirdPerson" 1 (struct)))

(event `ActivateRagdoll`
  ;[1 1 1] Enable Player Ragdoll
  (if (not (`self.Ragdoll`))
    (`PrimitiveComponent.SetCollisionEnabled` (`self.Mesh`) "QueryAndPhysics")
    (`PrimitiveComponent.SetSimulatePhysics` (`self.Mesh`) true)
    (`CharacterMovementComponent.DisableMovement` (`self.CharacterMovement`))
    (set `self.Ragdoll` true)
    (`GameplayStatics.PlaySound2D` "/Game/Sound/Sfx/wasted_sound.wasted_sound" 1.0 1.0 0.0 null null)
    (bind _returnvalue (`|CreateWidget` "/Game/Characters/Clementine/Interaction/WB_Wasted.WB_Wasted_C"))
    (`UserWidget.AddToViewport` _returnvalue 0)
    (`/Game/Characters/Clementine/Interaction/WB_Wasted.PlayWastedAnim` _returnvalue)
    (`PlayerCameraManager.StartCameraFade` :`self` (`GameplayStatics.GetPlayerCameraManager` 0) :`ToAlpha` 1.0 :`Duration` 4.0 :`bHoldWhenFinished` true)
    (`KismetSystemLibrary.Delay` 5.0)
    (`GameplayStatics.OpenLevelBySoftObjectPtr` "/Game/Levels/Test.Test")))

(event `Deactivate Ragdoll`
  (bind _capsulecomponent (`self.CapsuleComponent`))
  (bind (_returnvalue_roll _returnvalue_pitch _returnvalue_yaw) (`KismetMathLibrary.BreakRotator` (`SceneComponent.K2_GetComponentRotation` _capsulecomponent)))
  ;[1 1 1] Disable Regdoll
  (if (`self.Ragdoll`)
    (`PrimitiveComponent.SetSimulatePhysics` (`self.Mesh`) false)
    (set `self.Ragdoll` false)
    (`SceneComponent.K2_SetWorldLocationAndRotation` (`self.Mesh`) (- (`SceneComponent.K2_GetComponentLocation` _capsulecomponent) (0.0 0.0 97.0)) (`KismetMathLibrary.MakeRotator` _returnvalue_roll _returnvalue_pitch (- _returnvalue_yaw 90.0)) false false)
    (`SceneComponent.K2_AttachToComponent` (`self.Mesh`) (`self.CapsuleComponent`) "Hips" "KeepWorld" "KeepWorld" "KeepWorld" true)
    (`CharacterMovementComponent.SetMovementMode` (`self.CharacterMovement`) "MOVE_Walking" 0)
    (`Widget.RemoveFromParent` (stale `ActivateRagdoll` _returnvalue))))

(event `Key|R`
  (params (Key :type "Key Structure"))
  (:`Pressed`
    (`self.ActivateRagdoll`)))

(event `Key|Shift+R`
  (params (Key :type "Key Structure"))
  (:`Pressed`
    (`self.Deactivate Ragdoll`)))

(event `Key|K`
  (params (Key :type "Key Structure"))
  (:`Pressed`
    (bind _returnvalue (`GameplayStatics.GetActorOfClass` "/Game/Characters/NPC/AI2/NPCSpawner/BP_NPCSpawner.BP_NPCSpawner_C"))
    (`KismetSystemLibrary.PrintString` (`KismetStringLibrary.Conv_DoubleToString` (`KismetMathLibrary.Vector_Distance` (`self.K2_GetActorLocation` (`GameplayStatics.GetPlayerPawn` 0)) (`self.K2_GetActorLocation` _returnvalue))))))

(fn `IsPlayer?`
  (returns (`Yes/No` :type Boolean))
  (return (`self.IsPlayerControlled`)))

(fn `UserConstructionScript`)