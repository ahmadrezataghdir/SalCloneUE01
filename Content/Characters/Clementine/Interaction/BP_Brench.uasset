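; Interactable bench that seats the interacting character and stands them back up when the interaction ends.
; On start it plays a sit-idle montage, eases the capsule to a spot offset along world Y from the bench, turned 90 degrees from its yaw, and disables movement.
; On end it stops the montage, moves the character to the StandLocation component and restores walking.
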(event `self.Start Interaction`
  (bind (_returnvalue_roll _returnvalue_pitch _returnvalue_yaw) (`KismetMathLibrary.BreakRotator` (`self.K2_GetActorRotation`)))
  (bind _character (`self.Character`))
  (`parent.Start Interaction`)
  (bind _ascharacter (cast `Character` (`self.InteractingActor`)))
  (bind _output_get (set `self.Character` _ascharacter))
  (`Character.PlayAnimMontage` _output_get "/Game/Characters/Clementine/Anims/Re_SitIdle_Montage.Re_SitIdle_Montage" 1.0 "None")
  (`KismetSystemLibrary.MoveComponentTo` (`Actor.RootComponent` _character) (+ (`self.K2_GetActorLocation`) (`KismetMathLibrary.MakeVector` 0.0 50.0 (`CapsuleComponent.CapsuleHalfHeight` (`Character.CapsuleComponent` _character)))) (`KismetMathLibrary.MakeRotator` 0.0 0.0 (+ _returnvalue_yaw 90.0)) true true 0.5)
  (`CharacterMovementComponent.SetMovementMode` (`Character.CharacterMovement` (`self.Character`)) "MOVE_None" 0))

(event `self.End Interaction`
  (bind _character (`self.Character`))
  (`parent.End Interaction`)
  (bind _character_2 (`self.Character`)
    (:`then`
      (`Character.StopAnimMontage` _character_2 "/Game/Characters/Clementine/Anims/Re_SitIdle_Montage.Re_SitIdle_Montage")
      (`KismetSystemLibrary.MoveComponentTo` (`Actor.RootComponent` _character) (+ (`KismetMathLibrary.MakeVector` 0.0 0.0 (`CapsuleComponent.CapsuleHalfHeight` (`Character.CapsuleComponent` _character))) (`SceneComponent.K2_GetComponentLocation` (`self.StandLocation`))) (`self.K2_GetActorRotation` _character) false false 0.5)
      (`CharacterMovementComponent.SetMovementMode` (`Character.CharacterMovement` (`self.Character`)) "MOVE_Walking" 0))
    (:`else`)))

(fn `UserConstructionScript`
  (`parent.UserConstructionScript`))