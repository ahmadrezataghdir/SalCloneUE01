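; Rideable scooter pawn for Clementine that drives forward-only and ragdolls NPCs it hits above a speed threshold.
; Interaction seats the character on a socket with hand IK, idle montage and speedometer widget; ending restores walking, and E repossesses Clementine.
; Enhanced Input steers the FloatingPawnMovement and toggles engine audio.
; An interpolated throttle scales movement and lights, and drives the displayed speed instead of actual velocity.
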(event `self.ReceiveBeginPlay`
  (bind _floatingpawnmovement (`self.FloatingPawnMovement`))
  (`parent.ReceiveBeginPlay`)
  (set `FloatingPawnMovement.MaxSpeed` (* (`self.MaxSpeedKmh`) 27.7778) _floatingpawnmovement)
  (set `FloatingPawnMovement.Acceleration` (`self.Accel`) _floatingpawnmovement)
  (set `FloatingPawnMovement.Deceleration` (`self.Decel`) _floatingpawnmovement)
  (set `FloatingPawnMovement.TurningBoost` 0.0 _floatingpawnmovement))

(event `self.ReceiveTick`
  (params (DeltaSeconds :type "Float (single-precision)"))
  (bind _throttle_target (`self.Get ThrottleTarget` (`self.ForwardAxis`)))
  (bind _returnvalue (* (`self.Throttle_Current`) 10.0))
  (`parent.ReceiveTick` DeltaSeconds)
  (`self.SetScooterUIText` DeltaSeconds)
  (set `self.Throttle_Current` (`KismetMathLibrary.FInterpTo` (`self.Throttle_Current`) _throttle_target (`GameplayStatics.GetWorldDeltaSeconds`) (`self.Rate` _throttle_target (`self.Throttle_Current`))))
  (`LightComponent.SetIntensity` (`self.BackLight`) _returnvalue)
  (`LightComponent.SetIntensity` (`self.FrontLight`) _returnvalue))

(event `self.Start Interaction`
  (bind (_returnvalue_roll _returnvalue_pitch _returnvalue_yaw) (`KismetMathLibrary.BreakRotator` (`self.K2_GetActorRotation`)))
  (bind _character (`self.Character`))
  (bind _character_2 (`self.Character`))
  ;[1 1 1] Start Idle Anim, Setting hand ik, Removing foot ik, setting char pos in scooter, Disable movement, collision and attach char to scooter.
  (`parent.Start Interaction`)
  (bind _ascharacter (cast `Character` (`self.InteractingActor`)))
  (bind _output_get (set `self.Character` _ascharacter))
  (bind _asabp_clem (cast `/Game/Characters/Clementine/Blueprints/ABP_Clem` (`SkeletalMeshComponent.GetAnimInstance` (`Character.Mesh` _output_get))))
  (set `/Game/Characters/Clementine/Blueprints/ABP_Clem.HandIkAlpha` 1.0 _asabp_clem)
  (set `/Game/Characters/Clementine/Blueprints/ABP_Clem.FootAlpha` 0.01 _asabp_clem)
  (`Character.PlayAnimMontage` _output_get "/Game/Characters/Clementine/Anims/R_MF_Idle_Montage.R_MF_Idle_Montage" 1.0 "None")
  (`KismetSystemLibrary.MoveComponentTo` (`Actor.RootComponent` _character_2) (+ (`self.K2_GetActorLocation`) (`KismetMathLibrary.MakeVector` 0.0 0.0 (- (`CapsuleComponent.CapsuleHalfHeight` (`Character.CapsuleComponent` _character_2)) 6.5))) (`KismetMathLibrary.MakeRotator` 0.0 0.0 (+ _returnvalue_yaw 180.0)) true true 0.5)
  (`CharacterMovementComponent.SetMovementMode` (`Character.CharacterMovement` _character) "MOVE_None" 0)
  (`self.SetActorEnableCollision` _character false)
  (`GameplayStatics.GetActorOfClass` "BP_PawnScooter_C")
  (`self.K2_AttachToComponent` _character (`self.ScooterMesh`) "SeatSocket" "SnapToTarget" "SnapToTarget" "KeepRelative" true)
  (bind _returnvalue (`|CreateWidget` "/Game/Characters/Clementine/Interaction/ScooterSpeedoMeter.ScooterSpeedoMeter_C" (`GameplayStatics.GetPlayerController` 0)))
  (bind _output_get_2 (set `self.SpeedoMeterWidget` _returnvalue))
  (`UserWidget.AddToViewport` _output_get_2 0))

(event `self.End Interaction`
  (bind _character (`self.Character`))
  (bind _scooter_engine (`self.scooter_engine`))
  (bind _character_2 (`self.Character`))
  ;[1 1 1] Stop Animation, Getting character out of scooter, Enable Movement, Collision and Detaching from scooter.
  (`parent.End Interaction`)
  (bind _character_3 (`self.Character`)
    (:`then`
      (bind _asabp_clem (cast `/Game/Characters/Clementine/Blueprints/ABP_Clem` (`SkeletalMeshComponent.GetAnimInstance` (`Character.Mesh` _character_3))))
      (set `/Game/Characters/Clementine/Blueprints/ABP_Clem.HandIkAlpha` 0.0 _asabp_clem)
      (set `/Game/Characters/Clementine/Blueprints/ABP_Clem.FootAlpha` 1.0 _asabp_clem)
      (`Character.StopAnimMontage` _character_3 "/Game/Characters/Clementine/Anims/R_MF_Idle_Montage.R_MF_Idle_Montage")
      (`Widget.RemoveFromParent` (`self.SpeedoMeterWidget`))
      (`self.K2_SetActorTransform` _character_2 (`KismetMathLibrary.MakeTransform` (+ (`KismetMathLibrary.MakeVector` 0.0 0.0 (`CapsuleComponent.CapsuleHalfHeight` (`Character.CapsuleComponent` _character_2))) (`SceneComponent.K2_GetComponentLocation` (`self.StandLocation`))) (`self.K2_GetActorRotation` _character_2)) false false)
      (`CharacterMovementComponent.SetMovementMode` (`Character.CharacterMovement` _character) "MOVE_Walking" 0)
      (`self.SetActorEnableCollision` _character true)
      (`self.K2_DetachFromActor` _character "KeepWorld" "KeepWorld" "KeepWorld")
      (if (`AudioComponent.IsPlaying` _scooter_engine)
        (`AudioComponent.Stop` _scooter_engine)))
    (:`else`)))

(event `Key|E`
  (params (Key :type "Key Structure"))
  ;[1 1 1] Getting in Scooter, Start Sound and Cahning Controller To Scooter
  (:`Pressed`
    (bind _returnvalue (`GameplayStatics.GetActorOfClass` "/Game/Characters/Clementine/Blueprints/BP_Clem.BP_Clem_C"))
    (set `/Game/Characters/Clementine/Blueprints/BP_Clem.InsideScooter` false _returnvalue)
    (`GameplayStatics.PlaySound2D` "/Engine/VREditor/Sounds/UI/Camera_Shutter.Camera_Shutter" 1.0 1.0 0.0 null null)
    (`Controller.Possess` (`GameplayStatics.GetPlayerController` 0) _returnvalue)))

(event `start engine`
  ;[1 1 1] Engine Sound On
  (if (`self.enginePlaying`)
    (`AudioComponent.Play` (`self.scooter_engine`) 0.0)))

(event `EndEngine`
  ;[1 1 1] Engine Sound Off
  (`AudioComponent.Stop` (`self.scooter_engine`)))

(event `EnhancedInput|/Game/Characters/Clementine/Inputs/INP_ScooterMoveAround`
  (params (ActionValue :type "Vector2D Structure") (ElapsedSeconds :type "Float (double-precision)") (TriggeredSeconds :type "Float (double-precision)") (InputAction :type "InputAction Object Reference" :default "/Game/Characters/Clementine/Inputs/INP_ScooterMoveAround.INP_ScooterMoveAround"))
  (bind (_returnvalue_roll _returnvalue_pitch _returnvalue_yaw) (`KismetMathLibrary.BreakRotator` (`self.GetControlRotation`)))
  (bind _scooter_engine (`self.scooter_engine`))
  (bind _scooter_engine_2 (`self.scooter_engine`))
  ;[1 1 1] Scooter Movement Foward Only
  (:`Triggered`
    (set `self.ForwardAxis` (`KismetMathLibrary.FClamp` ActionValue_Y))
    (`self.AddControllerYawInput` (* ActionValue_X (`self.TurnRate`) (`GameplayStatics.GetWorldDeltaSeconds`)))
    (`self.AddMovementInput` (`PawnMovementComponent.GetPawnOwner` (`self.FloatingPawnMovement`)) (`KismetMathLibrary.GetForwardVector` (`KismetMathLibrary.MakeRotator` 0.0 0.0 _returnvalue_yaw)) (`self.Throttle_Current`) false)
    ;[1 1 1] Playing Engine Sound
    (if (!= ActionValue_Y 0.0) :!label _label
      (if (not (`self.enginePlaying`))
        (set `self.enginePlaying` true)
        (if (not (`AudioComponent.IsPlaying` _scooter_engine))
          (`AudioComponent.Play` _scooter_engine 0.0)))
      (elif (`self.enginePlaying`)
        (set `self.enginePlaying` false)
        (if (`AudioComponent.IsPlaying` _scooter_engine_2)
          (`AudioComponent.Stop` _scooter_engine_2)))))
  (:`Completed`
    (set `self.ForwardAxis` 0.0)
    (goto _label)))

(event `EnhancedInput|/Game/Characters/Clementine/Inputs/INP_ScooterLookAround`
  (params (ActionValue :type "Vector2D Structure") (ElapsedSeconds :type "Float (double-precision)") (TriggeredSeconds :type "Float (double-precision)") (InputAction :type "InputAction Object Reference" :default "/Game/Characters/Clementine/Inputs/INP_ScooterLookAround.INP_ScooterLookAround"))
  (bind _returnvalue (`PawnMovementComponent.GetPawnOwner` (`self.FloatingPawnMovement`)))
  ;[1 1 1] Scooter LookAround
  (:`Triggered`
    (`self.AddControllerYawInput` _returnvalue (* ActionValue_X (`KismetMathLibrary.SelectFloat` -1.0 1.0 (`self.InvertCameraX`))))
    (`self.AddControllerPitchInput` _returnvalue (* ActionValue_Y (`KismetMathLibrary.SelectFloat` -1.0 1.0 (`self.InvertCameraY`))))))

(event `self.CapsuleComponent.OnComponentHit`
  (params (HitComponent :type "PrimitiveComponent Object Reference") (OtherActor :type "Actor Object Reference") (OtherComp :type "PrimitiveComponent Object Reference") (NormalImpulse :type "Vector Structure") (Hit :type "HitResult Structure (by ref)"))
  ;[1 1 1] Make Hit By Scooter if speed greater than 15KMPH
  (bind _asbp_npc_m (cast `/Game/Characters/NPC/AI2/Blueprints/BP_NPC_M` OtherActor))
  (if (> (`self.SpeedKmh_Display`) 20.0)
    (`/Game/Characters/NPC/AI2/Blueprints/BP_NPC_M.ActivateRagdoll` _asbp_npc_m (`ActorComponent.GetOwner` (`self.ScooterMesh`)))))

(fn `GetSpeedInKMH`
  (returns (Speed :type "Float (double-precision)"))
  (return (* (`KismetMathLibrary.VSizeXY` (`self.GetVelocity` self)) 0.036)))

(fn `Set Speed to UI`
  (params (DeltaTime :type "Float (double-precision)"))
  (returns (Speed :type "Float (double-precision)"))
  (bind _maxspeedkmh (`self.MaxSpeedKmh`))
  (return (`KismetMathLibrary.FInterpTo` (`self.SpeedKmh_Display`) (* (`KismetMathLibrary.FClamp` (`self.Throttle_Current`)) _maxspeedkmh) DeltaTime (/ _maxspeedkmh 0.4))))

(fn `SetScooterUIText`
  (params (DeltaTime :type "Float (double-precision)"))
  (bind _speed (`self.Set Speed to UI` DeltaTime))
  (bind _speedometerwidget (`self.SpeedoMeterWidget`))
  (`/Engine/EditorBlueprintResources/StandardMacros.IsValid` _speedometerwidget
    (:`Is Valid`
      (bind _output_get (set `self.SpeedKmh_Display` _speed))
      (set `TextBlock.Text` (select `bool` (> _output_get 0.0) :`false` "N/A" :`true` (`KismetTextLibrary.Conv_DoubleToText` _output_get "HalfToEven" false true 1 3 0 2)) (`/Game/Characters/Clementine/Interaction/ScooterSpeedoMeter.ESpeed` _speedometerwidget))
      (`Widget.SetRenderTransformAngle` (`/Game/Characters/Clementine/Interaction/ScooterSpeedoMeter.SpeedoMeterGage` _speedometerwidget) (* _speed -3.0)))))

(fn `UserConstructionScript`
  (`parent.UserConstructionScript`))