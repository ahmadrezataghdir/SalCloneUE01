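; BP_Statue is an interactable statue that summons the nearest BP_NPC_M to the interacting character for a timed interaction.
; On start it locks re-entry with BlockKey, freezes the character's movement and sends the closest NPC over with AI MoveTo.
; On arrival it signals the NPC through BPI_Character, then after a fixed delay stops it, restores walking and calls the parent's EndInteraction.
; Its own EndInteraction is empty, leaving the montage-stop cleanup disconnected.
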(event `self.Start Interaction`
  (bind _nearestnpc (`self.NearestNPC`))
  (`parent.Start Interaction`)
  (if (`self.BlockKey`)
    (`KismetSystemLibrary.PrintString` "Interaction Already Started")
    (else
      (set `self.BlockKey` true)
      (bind _ascharacter (cast `Character` (`self.InteractingActor`)))
      (bind _output_get (set `self.Character` _ascharacter))
      (bind _outactors (`GameplayStatics.GetAllActorsOfClass` "/Game/Characters/NPC/AI2/Blueprints/BP_NPC_M.BP_NPC_M_C"))
      (for _array_element _outactors
        (bind _returnvalue (`KismetMathLibrary.Vector_Distance` (`self.K2_GetActorLocation` _array_element) (`self.K2_GetActorLocation` _output_get)))
        (if (< _returnvalue (`self.MinDistance`))
          (set `self.MinDistance` _returnvalue)
          (set `self.NearestNPC` _array_element)))
      (`CharacterMovementComponent.SetMovementMode` (`Character.CharacterMovement` (`self.Character`)) "MOVE_None" 0)
      (`AITask_MoveTo.AIMoveTo` (`AIBlueprintHelperLibrary.GetAIController` _nearestnpc) (0.0 0.0 0.0) (`self.Character`) -1.0 "Enable"
        (:`OnMoveFinished`
          (if (`KismetSystemLibrary.DoesImplementInterface` _nearestnpc "/Game/Characters/Clementine/Interface/BPI_Character.BPI_Character_C")
            (message `/Game/Characters/Clementine/Interface/BPI_Character.InteractStart` _nearestnpc)
            (`KismetSystemLibrary.Delay` 30.0)
            (if (`KismetSystemLibrary.DoesImplementInterface` _nearestnpc "/Game/Characters/Clementine/Interface/BPI_Character.BPI_Character_C")
              (message `/Game/Characters/Clementine/Interface/BPI_Character.InteractStop` _nearestnpc)
              (`CharacterMovementComponent.SetMovementMode` (`Character.CharacterMovement` (`self.Character`)) "MOVE_Walking" 0)
              (set `self.BlockKey` false)
              (`parent.End Interaction`))))))))

(event `self.End Interaction`)

(fn `UserConstructionScript`
  (`parent.UserConstructionScript`))