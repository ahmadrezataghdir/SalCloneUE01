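; Base interactable pawn that lets Clem interact with it, with scooter-specific hooks such as the InsideScooter flag and an empty MountScooter event.
; Box overlap with the player registers it as Clem's CurrentInteractable, shows an instruction widget and enables input, then reverses this on exit.
; Possession or StartInteract sets the interacting state and hides the prompt when starting, while unpossession clears that state.
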(event `self.Box.OnComponentBeginOverlap`
  (params (OverlappedComponent :type "PrimitiveComponent Object Reference") (OtherActor :type "Actor Object Reference") (OtherComp :type "PrimitiveComponent Object Reference") (OtherBodyIndex :type Integer) (bFromSweep :type Boolean) (SweepResult :type "HitResult Structure (by ref)"))
  (bind _yes_no (message `/Game/Characters/Clementine/Interface/BPI_Character.IsPlayer?` OtherActor))
  (if _yes_no
    (set `self.InteractingActor` OtherActor)
    (bind _asbp_clem (cast `/Game/Characters/Clementine/Blueprints/BP_Clem` (`self.InteractingActor`)))
    (set `/Game/Characters/Clementine/Blueprints/BP_Clem.InsideScooter` true _asbp_clem)
    (`self.WDGInstruction`
      (:`then`
        _)
      (:`else`
        (bind _returnvalue (`|CreateWidget` "/Game/Characters/Clementine/Interaction/WDG_Instruction.WDG_Instruction_C"))
        (set `self.WDGInstruction` _returnvalue)))
    (`UserWidget.AddToViewport` (`self.WDGInstruction`) 0)
    (`self.EnableInput` (`GameplayStatics.GetPlayerController` 0))
    (set `/Game/Characters/Clementine/Blueprints/BP_Clem.CurrentInteractable` self _asbp_clem)))

(event `self.Box.OnComponentEndOverlap`
  (params (OverlappedComponent :type "PrimitiveComponent Object Reference") (OtherActor :type "Actor Object Reference") (OtherComp :type "PrimitiveComponent Object Reference") (OtherBodyIndex :type Integer))
  (bind _yes_no (message `/Game/Characters/Clementine/Interface/BPI_Character.IsPlayer?` OtherActor))
  (if _yes_no
    (bind _asbp_clem (cast `/Game/Characters/Clementine/Blueprints/BP_Clem` (`self.InteractingActor`)))
    (set `/Game/Characters/Clementine/Blueprints/BP_Clem.InsideScooter` false _asbp_clem)
    (`self.HideInstruction`)
    (`self.DisableInput` (`GameplayStatics.GetPlayerController` 0))
    (set `/Game/Characters/Clementine/Blueprints/BP_Clem.CurrentInteractable` null _asbp_clem)))

(event `self.ReceivePossessed`
  (params (NewController :type "Controller Object Reference"))
  (`self.Start Interaction`))

(event `self.ReceiveUnpossessed`
  (params (OldController :type "Controller Object Reference"))
  (`self.End Interaction`))

(event `Start Interaction`
  (set `self.Interactiong` true)
  (`self.HideInstruction`))

(event `End Interaction`
  (set `self.Interactiong` false))

(event `Mount Scooter`)

(fn `StartInteract`
  (params (interact :type Boolean))
  (if interact
    (`self.Start Interaction`)
    (else
      (`self.End Interaction`))))

(fn `UserConstructionScript`)