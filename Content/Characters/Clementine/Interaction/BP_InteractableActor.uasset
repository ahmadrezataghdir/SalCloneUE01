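; BP_InteractableActor is an interactable world object that shows an instruction prompt when the player enters its Box trigger.
; Overlap identifies the player via IsPlayerMessage, stores the actor, displays a lazily created, reused WDG_Instruction and enables input; leaving reverses prompt and input.
; E toggles StartInteraction and EndInteraction through a flag.
; Both events are skeletal: starting hides the prompt and prints a debug string, while ending only clears the flag.
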(event `self.Box.OnComponentBeginOverlap`
  (params (OverlappedComponent :type "PrimitiveComponent Object Reference") (OtherActor :type "Actor Object Reference") (OtherComp :type "PrimitiveComponent Object Reference") (OtherBodyIndex :type Integer) (bFromSweep :type Boolean) (SweepResult :type "HitResult Structure (by ref)"))
  ;[1 1 1] Within object range
  (bind _yes_no (message `/Game/Characters/Clementine/Interface/BPI_Character.IsPlayer?` OtherActor))
  (if _yes_no
    (set `self.InteractingActor` OtherActor)
    (`self.WDGInstruction`
      (:`then`
        _)
      (:`else`
        (bind _returnvalue (`|CreateWidget` "/Game/Characters/Clementine/Interaction/WDG_Instruction.WDG_Instruction_C"))
        (set `self.WDGInstruction` _returnvalue)))
    (`UserWidget.AddToViewport` (`self.WDGInstruction`) 0)
    (`self.EnableInput` (`GameplayStatics.GetPlayerController` 0))))

(event `self.Box.OnComponentEndOverlap`
  (params (OverlappedComponent :type "PrimitiveComponent Object Reference") (OtherActor :type "Actor Object Reference") (OtherComp :type "PrimitiveComponent Object Reference") (OtherBodyIndex :type Integer))
  ;[1 1 1] Out of object range
  (bind _yes_no (message `/Game/Characters/Clementine/Interface/BPI_Character.IsPlayer?` OtherActor))
  (if _yes_no
    (`self.HideInstruction`)
    (`self.DisableInput` (`GameplayStatics.GetPlayerController` 0))))

(event `Key|E`
  (params (Key :type "Key Structure"))
  (:`Pressed`
    (if (`self.Interactiong`)
      (`self.End Interaction`)
      (else
        (`self.Start Interaction`)))))

(event `Start Interaction`
  (set `self.Interactiong` true)
  (`self.HideInstruction`)
  (`KismetSystemLibrary.PrintString` "Interacting"))

(event `End Interaction`
  (set `self.Interactiong` false))

(fn `UserConstructionScript`)