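; Fire alarm actor that, on interaction, toggles guidance for safety items and fire exits in the level.
; Interact flip-flops between Show and Hide, which set an outline stencil on "safe"-tagged Safety_ actors and toggle the Exit component's visibility on every FireExit_bp.
; Box overlap sets the alarm mesh's custom depth stencil as a highlight, only when the overlapping actor's instigator is locally controlled.
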(event `/Game/Hosting/PlatformContent/InteractInterface.Interact`
  (params (`Actor to Interact` :type "Actor Object Reference"))
  (`/Engine/EditorBlueprintResources/StandardMacros.FlipFlop`
    (:`A`
      (`self.Show`))
    (:`B`
      (`self.Hide`))))

(event `self.Box.OnComponentBeginOverlap`
  (params (OverlappedComponent :type "PrimitiveComponent Object Reference") (OtherActor :type "Actor Object Reference") (OtherComp :type "PrimitiveComponent Object Reference") (OtherBodyIndex :type Integer) (bFromSweep :type Boolean) (SweepResult :type "HitResult Structure (by ref)"))
  (if (`Pawn.IsLocallyControlled` (`Actor.Instigator` OtherActor))
    (`PrimitiveComponent.SetCustomDepthStencilValue` (`self.Alarrm`) 2)))

(event `Hide`
  (`self.Hide_Outline`)
  (`self.HideExit`))

(event `Show`
  (`self.Show_Outline`)
  (`self.ShowExit`))

(event `self.Box.OnComponentEndOverlap`
  (params (OverlappedComponent :type "PrimitiveComponent Object Reference") (OtherActor :type "Actor Object Reference") (OtherComp :type "PrimitiveComponent Object Reference") (OtherBodyIndex :type Integer))
  (if (`Pawn.IsLocallyControlled` (`Actor.Instigator` OtherActor))
    (`PrimitiveComponent.SetCustomDepthStencilValue` (`self.Alarrm`) 0)))

(event `Hide_Outline`
  ;[0 1 0.3774] Outline
  (bind _outactors (`GameplayStatics.GetAllActorsOfClassWithTag` "/Game/Blueprints/Fire/Safety_.Safety__C" "safe"))
  (for _array_element _outactors
    (`PrimitiveComponent.SetCustomDepthStencilValue` (`/Game/Blueprints/Fire/Safety_.Mesh` _array_element) 0)))

(event `Show_Outline`
  ;[0 1 0.3774] Outline
  (bind _outactors (`GameplayStatics.GetAllActorsOfClassWithTag` "/Game/Blueprints/Fire/Safety_.Safety__C" "safe"))
  (for _array_element _outactors
    (`PrimitiveComponent.SetCustomDepthStencilValue` (`/Game/Blueprints/Fire/Safety_.Mesh` _array_element) 2)))

(event `ShowExit`
  ;[0 1 0.3774] Outline
  (bind _outactors (`GameplayStatics.GetAllActorsOfClass` "/Game/Blueprints/Fire/FireExits/FireExit_bp.FireExit_bp_C"))
  (for _array_element _outactors
    (`SceneComponent.SetVisibility` (`/Game/Blueprints/Fire/FireExits/FireExit_bp.Exit` _array_element) true false)))

(event `HideExit`
  ;[0 1 0.3774] Outline
  (bind _outactors (`GameplayStatics.GetAllActorsOfClass` "/Game/Blueprints/Fire/FireExits/FireExit_bp.FireExit_bp_C"))
  (for _array_element _outactors
    (`SceneComponent.SetVisibility` (`/Game/Blueprints/Fire/FireExits/FireExit_bp.Exit` _array_element) false false)))

(fn `UserConstructionScript`)