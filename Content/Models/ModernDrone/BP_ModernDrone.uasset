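; Flyable drone pawn that the player possesses when activated and leaves with F, swapping in a drone HUD.
; A proximity trigger shows the interaction prompt and flags BP_Clem as nearby.
; Enhanced Input drives FloatingPawnMovement, yaw and scene-capture pitch; up-input when grounded assembles the drone through its AnimBP.
; While possessed, Tick line-traces altitude and camera distance, auto-disassembling near the ground; helper functions compute spin and steering values.
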(event `self.ReceiveBeginPlay`)

(event `self.ReceiveActorBeginOverlap`
  (params (OtherActor :type "Actor Object Reference"))
  (`KismetSystemLibrary.PrintString` (`KismetSystemLibrary.GetDisplayName` OtherActor)))

(event `ShowInteractionText`
  (params (Show :type Boolean))
  (bind _widget (`self.Widget`))
  (bind _returnvalue (`WidgetComponent.GetUserWidgetObject` _widget))
  (if Show
    (bind _asinteraction_prompt (cast `/Game/Characters/Clementine/Interaction/InteractionPrompt` _returnvalue))
    (`Image.SetBrushFromTexture` (`/Game/Characters/Clementine/Interaction/InteractionPrompt.EImage` _asinteraction_prompt) "/Game/Characters/Clementine/Interaction/Fe.Fe" false)
    (`TextBlock.SetText` (`/Game/Characters/Clementine/Interaction/InteractionPrompt.EText` _asinteraction_prompt) "F To Activate. T to Start.")
    (`SceneComponent.SetVisibility` _widget true false)
    (else
      (bind _asinteraction_prompt_2 (cast `/Game/Characters/Clementine/Interaction/InteractionPrompt` _returnvalue))
      (`Image.SetBrushFromTexture` (`/Game/Characters/Clementine/Interaction/InteractionPrompt.EImage` _asinteraction_prompt_2) "/Game/Characters/Clementine/Interaction/Fe.Fe" false)
      (`SceneComponent.SetVisibility` _widget false false))))

(event `self.PlayerTrigger.OnComponentBeginOverlap`
  (params (OverlappedComponent :type "PrimitiveComponent Object Reference") (OtherActor :type "Actor Object Reference") (OtherComp :type "PrimitiveComponent Object Reference") (OtherBodyIndex :type Integer) (bFromSweep :type Boolean) (SweepResult :type "HitResult Structure (by ref)"))
  (bind _yes_no (message `/Game/Characters/Clementine/Interface/BPI_Character.IsPlayer?` OtherActor))
  (if _yes_no
    (bind _asbp_clem (cast `/Game/Characters/Clementine/Blueprints/BP_Clem` OtherActor))
    (set `/Game/Characters/Clementine/Blueprints/BP_Clem.Is Drone Narby?` true _asbp_clem)
    (`self.ShowInteractionText` true)))

(event `self.PlayerTrigger.OnComponentEndOverlap`
  (params (OverlappedComponent :type "PrimitiveComponent Object Reference") (OtherActor :type "Actor Object Reference") (OtherComp :type "PrimitiveComponent Object Reference") (OtherBodyIndex :type Integer))
  (bind _yes_no (message `/Game/Characters/Clementine/Interface/BPI_Character.IsPlayer?` OtherActor))
  (if _yes_no
    (bind _asbp_clem (cast `/Game/Characters/Clementine/Blueprints/BP_Clem` OtherActor))
    (set `/Game/Characters/Clementine/Blueprints/BP_Clem.Is Drone Narby?` false _asbp_clem)
    (`self.ShowInteractionText` false)))

(event `EnhancedInput|/Game/Characters/Clementine/Inputs/INP_DroneDown`
  (params (ActionValue :type "Float (double-precision)") (ElapsedSeconds :type "Float (double-precision)") (TriggeredSeconds :type "Float (double-precision)") (InputAction :type "InputAction Object Reference" :default "/Game/Characters/Clementine/Inputs/INP_DroneDown.INP_DroneDown"))
  (:`Triggered`
    (if (not (`self.bIsGrounded`))
      (set `self.LiftInput` ActionValue)
      (`PawnMovementComponent.AddInputVector` (`self.FloatingPawnMovement`) (* (`KismetMathLibrary.Vector_Up`) ActionValue) false))))

(event `EnhancedInput|/Game/Characters/Clementine/Inputs/INP_DroneUp`
  (params (ActionValue :type "Float (double-precision)") (ElapsedSeconds :type "Float (double-precision)") (TriggeredSeconds :type "Float (double-precision)") (InputAction :type "InputAction Object Reference" :default "/Game/Characters/Clementine/Inputs/INP_DroneUp.INP_DroneUp"))
  (:`Triggered`
    (if (`self.bIsGrounded`)
      (`self.CallDroneAssemble`)
      (else
        (set `self.LiftInput` ActionValue)
        (`PawnMovementComponent.AddInputVector` (`self.FloatingPawnMovement`) (* (`KismetMathLibrary.Vector_Up`) ActionValue) false)))))

(event `EnhancedInput|/Game/Characters/Clementine/Inputs/INP_DroneMoveAround`
  (params (ActionValue :type "Vector2D Structure") (ElapsedSeconds :type "Float (double-precision)") (TriggeredSeconds :type "Float (double-precision)") (InputAction :type "InputAction Object Reference" :default "/Game/Characters/Clementine/Inputs/INP_DroneMoveAround.INP_DroneMoveAround"))
  (bind _floatingpawnmovement (`self.FloatingPawnMovement`))
  (:`Triggered`
    (if (`self.Assembled`)
      (if (not (`self.bIsGrounded`))
        (bind _output_get (set `self.ForwardInput` ActionValue_Y))
        (bind _output_get_2 (set `self.RightInput` ActionValue_X))
        (`PawnMovementComponent.AddInputVector` _floatingpawnmovement (* (`self.GetActorRightVector`) _output_get_2) false)
        (`PawnMovementComponent.AddInputVector` _floatingpawnmovement (* (`self.GetActorForwardVector`) _output_get) false))))
  (:`Completed`
    (set `self.ForwardInput` 0.0)
    (`KismetSystemLibrary.PrintString` (`KismetStringLibrary.Conv_DoubleToString` (`self.ForwardInput`)))))

(event `EnhancedInput|/Game/Characters/Clementine/Inputs/INP_DroneLookAround`
  (params (ActionValue :type "Vector2D Structure") (ElapsedSeconds :type "Float (double-precision)") (TriggeredSeconds :type "Float (double-precision)") (InputAction :type "InputAction Object Reference" :default "/Game/Characters/Clementine/Inputs/INP_DroneLookAround.INP_DroneLookAround"))
  (bind _scenecapturecomponent2d (`self.SceneCaptureComponent2D`))
  (bind (_relativerotation_roll _relativerotation_pitch) (`KismetMathLibrary.BreakRotator` (`SceneComponent.RelativeRotation` _scenecapturecomponent2d)))
  (:`Triggered`
    (if (`self.Assembled`)
      (if (not (`self.bIsGrounded`))
        (bind _output_get (set `self.YawInput` ActionValue_X))
        (`self.AddControllerYawInput` _output_get)
        (`SceneComponent.K2_SetRelativeRotation` _scenecapturecomponent2d (`KismetMathLibrary.MakeRotator` 0.0 (`KismetMathLibrary.FClamp` (+ (* ActionValue_Y -1.0) _relativerotation_pitch) -90.0 -10.0)) false false)))))

(event `Key|F`
  (params (Key :type "Key Structure"))
  (:`Pressed`
    (bind _asbp_clem (cast `/Game/Characters/Clementine/Blueprints/BP_Clem` (`self.PlayerPawn`)))
    (if (`/Game/Characters/Clementine/Blueprints/BP_Clem.Is Drone Narby?` _asbp_clem)
      (`self.Return Control`)
      (`KismetSystemLibrary.PrintString` (`KismetStringLibrary.Conv_DoubleToString` (`self.Spin_Current`)))
      (else
        (`KismetSystemLibrary.PrintString` "Not in range")))))

(event `CallDroneDisAssemble`
  (if (and (< (`self.AltitudeInMeters`) 0.3) (`self.Assembled`))
    (bind _asdrone_anim_blueprint (cast `/Game/Models/ModernDrone/Assets/DroneAnimBlueprint` (`SkeletalMeshComponent.GetAnimInstance` (`self.SkeletalMesh`))))
    (set `/Game/Models/ModernDrone/Assets/DroneAnimBlueprint.AssembleNow` false _asdrone_anim_blueprint)
    (`GameplayStatics.PlaySound2D` "/Engine/EditorSounds/Notifications/CompileStart_Cue.CompileStart_Cue" 1.0 1.0 0.0 null null)
    (`LightComponent.SetIntensity` (`self.SpotLight`) 0.0)
    (`SceneComponent.SetVisibility` (`self.Right`) false false)
    (`SceneComponent.SetVisibility` (`self.Left`) false false)
    (set `self.Assembled` false)))

(event `Return Control`
  (`self.DeactivateDrone`))

(event `self.ReceiveTick`
  (params (DeltaSeconds :type "Float (single-precision)"))
  (bind _returnvalue (`self.K2_GetActorLocation`))
  (bind _scenecapturecomponent2d (`self.SceneCaptureComponent2D`))
  (bind _audio (`self.Audio`))
  (bind _returnvalue_2 (`SceneComponent.K2_GetComponentLocation` _scenecapturecomponent2d))
  (switch `/Game/Models/ModernDrone/EDroneState` (`self.DroneStates`)
    (:`NewEnumerator1`
      (`|ExecutionSequence`
        (:`then_0`
          (bind (_outhit _returnvalue_3) (`KismetSystemLibrary.LineTraceSingle` _returnvalue (- _returnvalue (0.0 0.0 10000.0)) "TraceTypeQuery2"))
          (bind _output_get (set `self.AltitudeInMeters` (select `bool` _returnvalue_3 :`false` -1.0 :`true` (/ (`.Distance` (`GameplayStatics.BreakHitResult` _outhit)) 100.0))))
          (if (< _output_get 0.15)
            (bind _output_get_2 (set `self.bIsGrounded` true))
            (`AudioComponent.SetPaused` _audio _output_get_2)
            (`self.CallDroneDisAssemble`)
            (else
              (bind _output_get_3 (set `self.bIsGrounded` false))
              (`AudioComponent.SetPaused` _audio _output_get_3))))
        (:`then_1`
          (bind (_outhit_2 _returnvalue_4) (`KismetSystemLibrary.LineTraceSingle` _returnvalue_2 (+ _returnvalue_2 (* (`SceneComponent.GetForwardVector` _scenecapturecomponent2d) 10000.0)) "TraceTypeQuery2"))
          (set `self.DistanceInMeters` (select `bool` _returnvalue_4 :`false` -1.0 :`true` (/ (`.Distance` (`GameplayStatics.BreakHitResult` _outhit_2)) 100.0))))))))

(event `CallDroneAssemble`
  (bind _returnvalue (`self.K2_GetActorLocation`))
  (if (and (< (`self.AltitudeInMeters`) 0.2) (not (`self.Assembled`)))
    (bind _asdrone_anim_blueprint (cast `/Game/Models/ModernDrone/Assets/DroneAnimBlueprint` (`SkeletalMeshComponent.GetAnimInstance` (`self.SkeletalMesh`))))
    (set `/Game/Models/ModernDrone/Assets/DroneAnimBlueprint.AssembleNow` true _asdrone_anim_blueprint)
    (`GameplayStatics.PlaySound2D` "/Engine/EditorSounds/Notifications/CompileStart_Cue.CompileStart_Cue" 1.0 1.0 0.0 null null)
    (`KismetSystemLibrary.Delay` 0.0)
    (bind (_sweephitresult _returnvalue_2) (`self.K2_SetActorLocation` (`KismetMathLibrary.VInterpTo` _returnvalue (+ _returnvalue (0.0 0.0 60.0)) (`GameplayStatics.GetWorldDeltaSeconds`) 15.0) true))
    (if _returnvalue_2
      (`LightComponent.SetIntensity` (`self.SpotLight`) 50000.0)
      (`SceneComponent.SetVisibility` (`self.Right`) true false)
      (`SceneComponent.SetVisibility` (`self.Left`) true false)
      (set `self.Assembled` true))))

(fn `ActivateDrone`
  (params (Interactor :type "Character Object Reference"))
  (locals (PlayerController :type "PlayerController Object Reference"))
  (`self.ShowInteractionText` false)
  (switch `/Game/Models/ModernDrone/EDroneState` (`self.DroneStates`)
    (:`NewEnumerator0`
      (bind _output_get (set `self.PlayerPawn` Interactor))
      (bind _asplayer_controller (cast `PlayerController` (`self.GetController` _output_get)))
      (bind _output_get_2 (set `local.PlayerController` _asplayer_controller))
      (bind _returnvalue (`|CreateWidget` "/Game/Models/ModernDrone/DroneWidget.DroneWidget_C" _output_get_2))
      (bind _output_get_3 (set `self.DroneWidget` _returnvalue))
      (`UserWidget.AddToViewport` _output_get_3 0)
      (`Controller.Possess` (`local.PlayerController`) self)
      (set `self.DroneStates` "NewEnumerator1")
      (`AudioComponent.Play` (`self.Audio`) 0.0))))

(fn `Control the Steering`
  (params (SteeringValue :type "Float (double-precision)"))
  (bind _asdrone_anim_blueprint (cast `/Game/Models/ModernDrone/Assets/DroneAnimBlueprint` (`SkeletalMeshComponent.GetAnimInstance` (`self.SkeletalMesh`))))
  (set `/Game/Models/ModernDrone/Assets/DroneAnimBlueprint.SteeringValue` SteeringValue _asdrone_anim_blueprint)
  (return))

(fn `DeactivateDrone`
  (switch `/Game/Models/ModernDrone/EDroneState` (`self.DroneStates`)
    (:`NewEnumerator1`
      (`AudioComponent.Stop` (`self.Audio`))
      (`Controller.Possess` (`self.GetController`) (`self.PlayerPawn`))
      (bind _output_get (set `self.PlayerPawn` null))
      (`Widget.RemoveFromParent` (`self.DroneWidget`))
      (set `self.DroneWidget` null)
      (set `self.DroneStates` "NewEnumerator0"))))

(fn `GetAltitudeInMeters`
  (returns (AltitudeInMeters :type "Float (double-precision)"))
  (return (`self.AltitudeInMeters`)))

(fn `GetDistanceInMeters`
  (returns (DistanceInMeters :type "Float (double-precision)"))
  (return (`self.DistanceInMeters`)))

(fn `GetSmoothSteeringValue`
  (params (DeltaTime :type "Float (double-precision)"))
  (returns (SteeringValue :type "Float (double-precision)"))
  (bind _steeringmax (`self.SteeringMax`))
  (return (`KismetMathLibrary.FInterpTo` (`self.SteeringCurrent`) (* (`KismetMathLibrary.FClamp` (`self.ForwardInput`) -1.0) _steeringmax) DeltaTime (/ _steeringmax (`self.SteeringInterpSpeed`)))))

(fn `IsVerticalOnly`
  (returns (VerticalOnly :type Boolean))
  (bind _verticaldeadzone (`self.VerticalDeadzone`))
  (return (and (< (`KismetMathLibrary.Abs` (`self.ForwardInput`)) _verticaldeadzone) (> (`KismetMathLibrary.Abs` (`self.LiftInput`)) _verticaldeadzone))))

(fn `SetSpinTarget`
  (returns (Speed :type "Float (double-precision)"))
  (return (`KismetMathLibrary.FClamp` (+ (* (`KismetMathLibrary.FClamp` (/ (`KismetMathLibrary.VSizeXY` (`self.GetVelocity`)) (`self.MaxSpeedForNorm`))) (`KismetMathLibrary.FClamp` (`self.ForwardInput`) -1.0) (`self.MoveSpinScale`) (`self.SpinMax`)) (* (`KismetMathLibrary.Abs` (`self.LiftInput`)) (`self.LiftSpinScale`) (`self.SpinMax`))) (* (`self.SpinMax`) -1.0) (`self.SpinMax`))))

(fn `UserConstructionScript`)